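; BP_Button_1 is an interactable push button that switches its connected actors on, then automatically off after two seconds.
; Interacting plays a timeline that dips the button top and, on its press event, toggles State, calling On or Off on each Connection.
; The top's material reflects State, and each change is sent to InputSync actors, which can push state back through SyncInputState.
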(event EventBeginPlay
  (CallFunction|UpdateLight))

(event Collision|EventActorBeginOverlap
  (params (OtherActor :type Actor%20Object%20Reference)))

(event EventTick
  (params (DeltaSeconds :type Float%20%28single-precision%29)))

(event EventInteractwith
  (bind _alpha (Timeline|Timeline_ButtonAnimation PlayFromStart)
    (:Update
      (Transformation|SetRelativeLocation (Variables|Default|GetSM_Button_Top) (Math|Vector|Lerp(Vector) "0, 0, 0" "0, 0,-5.000000" _alpha) false false))
    (:Button%20Press
      (if (Variables|Runtime|GetState)
        (CallFunction|SetStateOff)
        (CallFunction|UpdateLight)
        (CallFunction|SyncState)
        (else
          (CallFunction|SetStateon)
          (CallFunction|UpdateLight)
          (CallFunction|SyncState)
          (Utilities|FlowControl|Delay 2.0)
          (CallFunction|SetStateOff)
          (CallFunction|UpdateLight)
          (CallFunction|SyncState))))))

(event EventSyncInputState
  (params (State :type Boolean))
  (Variables|Runtime|SetState State)
  (CallFunction|UpdateLight))

(fn ConstructionScript)

(fn UpdateLight
  (Rendering|Material|SetMaterial (Variables|Default|GetSM_Button_Top) 0 (select (Variables|Runtime|GetState) "/Game/InteractionSystem/Assets/Materials/ProcGrid/MI_ProcGrid_OnLines.MI_ProcGrid_OnLines" "/Game/InteractionSystem/Assets/Materials/ProcGrid/MI_ProcGrid_OffLines.MI_ProcGrid_OffLines")))

(fn SyncState
  (for _array_element (Variables|Data|GetInput%20Sync)
    (Class|BPIInteraction|SyncInputState(Message) _array_element (Variables|Runtime|GetState))))

(fn SetStateon
  (Variables|Runtime|SetState true)
  (for _array_element (Variables|Data|GetConnections)
    (Default|On _array_element)))

(fn SetStateOff
  (Variables|Runtime|SetState false)
  (for _array_element (Variables|Data|GetConnections)
    (Default|Off _array_element)))

(fn GetFractureBool
  (return false))

(fn GetItemType
  (return "NewEnumerator0"))

(fn GetMesh
  (return 0))