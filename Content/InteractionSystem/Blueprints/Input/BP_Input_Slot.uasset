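; BP_Input_Slot is an interaction-system input that switches on when an accepted item is placed into its trigger volume.
; On overlap, it accepts only unfractured BPI_Interaction actors whose class is in AcceptableInputs, and only while its state is off.
; A valid item is dropped with zero velocity and slotted to the volume via messages, then the state turns on.
; A DoOnce blocks repeat slotting until UnSlotItem turns the state off and resets it.
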(event OnComponentBeginOverlap(TriggerVolume)
  (params (OverlappedComponent :type Primitive%20Component%20Object%20Reference) (OtherActor :type Actor%20Object%20Reference) (OtherComp :type Primitive%20Component%20Object%20Reference) (OtherBodyIndex :type Integer) (bFromSweep :type Boolean) (SweepResult :type Hit%20Result%20Structure%20%28by%20ref%29))
  (Utilities|CanSlotItem? OtherActor
    (:true
      (Utilities|FlowControl|DoOnce false
        (:Completed
          (Class|BPIInteraction|DropItem(Message) OtherActor "0, 0, 0" false)
          (Class|BPIInteraction|SlotItem(Message) OtherActor (Variables|Default|GetTrigger%20Volume))
          (if true
            (CallFunction|SetStateon)))))))

(event EventUnSlotItem
  (CallFunction|SetStateOff)
  (Utilities|FlowControl|DoOnce false) ; enters at Reset
)

(fn ConstructionScript)

(fn GetMesh
  (return 0))

(fn GetInteractionType
  (return))